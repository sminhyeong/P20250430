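; BP_PlayerState holds the player's runtime state: current HP and counts of collected red, blue and green boxes.
; InitializedState seeds CurState from its character data, and IsAlive checks for HP above zero.
; AddDamage and AddHeal change HP without clamping, then broadcast UpdateHp with current and max values.
; AddBoxCount increments the matching color up to a cap of three, broadcasting UpdateBoxCount on success.
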(fn ConstructionScript)

(fn InitializedState
  (Variables|Default|SetCurState (Utilities|Struct|MakeST_CurCharacter (.CharacterData (Utilities|Struct|BreakST_CurCharacter (Variables|Default|GetCurState))) (.Hp (Utilities|Struct|BreakST_Character (.CharacterData (Utilities|Struct|BreakST_CurCharacter (Variables|Default|GetCurState))))) (.IsAlive (Utilities|Struct|BreakST_Character (.CharacterData (Utilities|Struct|BreakST_CurCharacter (Variables|Default|GetCurState))))))))

(fn AddDamage
  (params (Damage :type Float%20%28double-precision%29))
  (bind _curstate (Variables|Default|GetCurState))
  (Utilities|Struct|SetmembersinST_CurCharacter (Variables|Default|GetCurState) (- (.curhp (Variables|Default|GetCurState)) Damage))
  (Default|CallEventDispatcherUpdateHp (.curhp _curstate) (.hp (.characterdata _curstate))))

(fn AddBoxCount
  (params (BoxType :type EN_ItempType%20Enum :default "NewEnumerator0"))
  (switch Utilities|FlowControl|Switch|SwitchonEN_ItempType BoxType
    (:NewEnumerator0
      (if (CallFunction|CanAddRedCount)
        (bind _output_get (Variables|Default|SetRedCount (+ (Variables|Default|GetRedCount) 1)))
        (LocalVariables|SetUpdateCount _output_get)
        (Default|CallEventDispatcherUpdateBoxCount BoxType (LocalVariables|GetUpdateCount) :!label _label)))
    (:NewEnumerator1
      (if (CallFunction|CanAddBlueCount)
        (bind _output_get_2 (Variables|Default|SetBlueCount (+ (Variables|Default|GetBlueCount) 1)))
        (LocalVariables|SetUpdateCount _output_get_2)
        (goto _label)))
    (:NewEnumerator2
      (if (CallFunction|CanAddGreenCount)
        (bind _output_get_3 (Variables|Default|SetGreenCount (+ (Variables|Default|GetGreenCount) 1)))
        (LocalVariables|SetUpdateCount _output_get_3)
        (goto _label)))))

(fn IsAlive
  (return (> (.curhp (Variables|Default|GetCurState)) 0.0)))

(fn AddHeal
  (params (B :type Float%20%28double-precision%29))
  (bind _curstate (Variables|Default|GetCurState))
  (Utilities|Struct|SetmembersinST_CurCharacter (Variables|Default|GetCurState) (+ (.curhp (Variables|Default|GetCurState)) B))
  (Default|CallEventDispatcherUpdateHp (.curhp _curstate) (.hp (.characterdata _curstate))))

(fn CanAddBlueCount
  (return (< (Variables|Default|GetBlueCount) 3)))

(fn CanAddRedCount
  (return (< (Variables|Default|GetRedCount) 3)))

(fn CanAddGreenCount
  (return (< (Variables|Default|GetGreenCount) 3)))