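; Player Blueprint that takes damage and uses items it overlaps, keeping its stats in BP_PlayerState.
; BeginPlay initializes that state and binds its HP and box-count dispatchers for the HUD, firing a zero-damage call after the HP binding.
; Damage goes straight to the state, while capsule overlaps pass the item's UseItem result to BPItemController.
; The controller's heal-box and color-box dispatchers are also bound at startup.
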(event OnComponentBeginOverlap(CapsuleComponent)
  (params (OverlappedComponent :type Primitive%20Component%20Object%20Reference) (OtherActor :type Actor%20Object%20Reference) (OtherComp :type Primitive%20Component%20Object%20Reference) (OtherBodyIndex :type Integer) (bFromSweep :type Boolean) (SweepResult :type Hit%20Result%20Structure%20%28by%20ref%29))
  (bind _asbp_item_base (Utilities|Casting|CastToBP_ItemBase OtherActor))
  (bind _item_data_member_var_0 (Default|UseItem _asbp_item_base))
  (Default|UseItem (Variables|Default|GetBP_ItemController) _item_data_member_var_0))

(event EventBeginPlay
  (CallFunction|InitializedState)
  (CallFunction|BindStatetoHud)
  (CallFunction|BindStatetoItemController))

(event Game|Damage|EventAnyDamage
  (params (Damage :type Float%20%28single-precision%29) (DamageType :type Damage%20Type%20Object%20Reference) (InstigatedBy :type Controller%20Object%20Reference) (DamageCauser :type Actor%20Object%20Reference))
  (Default|AddDamage (Variables|Default|GetState) Damage))

(fn ConstructionScript
  (|CallParentFunction))

(fn InitializedState
  (bind _asbp_player_state (Utilities|Casting|CastToBP_PlayerState (Game|GetPlayerState 0)))
  (bind _output_get (Variables|Default|SetState _asbp_player_state))
  (Default|InitializedState _output_get))

(fn BindStatetoHud
  (bind _state (Variables|Default|GetState))
  (bind _asbp_hud (Utilities|Casting|CastToBP_Hud (HUD|GetHUD (Game|GetPlayerController 0))))
  (Utilities|FlowControl|Sequence
    (:then_0
      (EventDispatchers|BindEventtoEventDispatcherUpdateHp _state (EventDispatchers|CreateEvent _asbp_hud :!event SetHp))
      (Default|AddDamage (Variables|Default|GetState) 0.0))
    (:then_1
      (EventDispatchers|BindEventtoEventDispatcherUpdateBoxCount _state (EventDispatchers|CreateEvent _asbp_hud :!event SetBoxCount)))))

(fn BindStatetoItemController
  (EventDispatchers|BindEventtoEventDispatcherUseHealBox (Variables|Default|GetBP_ItemController) (EventDispatchers|CreateEvent (Variables|Default|GetState) :!event AddHeal))
  (EventDispatchers|BindEventtoEventDispatcherUseColorBox (Variables|Default|GetBP_ItemController) (EventDispatchers|CreateEvent (Variables|Default|GetState) :!event AddBoxCount)))