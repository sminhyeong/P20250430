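; Player component that periodically spawns random monsters and items around its owner, using two looping timers.
; Monster rows from DT_Monster spawn with BT_Monster on a navmesh-projected point on a ring around the owner.
; Spawned monsters are tracked in SpawnCount, and the monster timer pauses at ten, with no resume in this component.
; Item rows from DT_Item spawn at random navigable points near the owner, receiving their row data.
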(event EventBeginPlay
  (Utilities|Time|SetTimerbyFunctionName 0 "DoMonsterSpawn" 1.0 true)
  (Utilities|Time|SetTimerbyFunctionName 0 "DoItemSpawn" 3.0 true))

(fn DoMonsterSpawn
  (if (< (Utilities|Array|Length (Variables|Default|GetSpawnCount)) 10)
    (bind _outrownames (DataTable|GetDataTableRowNames "/Game/BluePrints/Character/Monster/DT_Monster.DT_Monster"))
    (bind _returnvalue (Utilities|GetDataTableRow "/Game/BluePrints/Character/Monster/DT_Monster.DT_Monster" (.OutItem (Utilities|Array|Random _outrownames)))
      (:then
        (bind _output_get (LocalVariables|SetNewLocalVar (CallFunction|MakeSpawnLocation)))
        (if (.ReturnValue (AI|Navigation|ProjectPointtoNavigation _output_get 0 0 "0, 0, 0"))
          (bind _returnvalue_2 (AI|SpawnAIFromClass (.BaseClass (Utilities|Struct|BreakST_Character _returnvalue)) "/Game/BluePrints/Character/Monster/BT_Monster.BT_Monster" (.ProjectedLocation (AI|Navigation|ProjectPointtoNavigation _output_get 0 0 "0, 0, 0")) "0, 0, 0" false 0))
          (bind _asbp_monster_base (Utilities|Casting|CastToBP_MonsterBase _returnvalue_2)
            (:then
              (Utilities|Array|Add (Variables|Default|GetSpawnCount) _asbp_monster_base)
              (if (>= (Utilities|Array|Length (Variables|Default|GetSpawnCount)) 10)
                (Class|KismetSystemLibrary|PauseTimer 0 "DoMonsterSpawn")))
            (:CastFailed
              (Actor|DestroyActor _asbp_monster_base))))))))

(fn MakeSpawnLocation
  (bind _radius (Variables|Default|GetRadius))
  (bind _returnvalue (* _radius 3.141592))
  (bind _output_get (LocalVariables|SetRand (Math|Random|RandomFloatinRange 0.0 3.6e+02)))
  (return (+ (Math|Vector|MakeVector (* (Math|Trig|Cos(Radians) _output_get) _returnvalue) (* (Math|Trig|Sin(Radians) _output_get) _returnvalue) 0.0) (Transformation|GetActorLocation (Components|GetOwner)))))

(fn DoItemSpawn
  (bind _outrownames (DataTable|GetDataTableRowNames "/Game/BluePrints/Item/DT_Item.DT_Item"))
  (bind _returnvalue (Utilities|GetDataTableRow "/Game/BluePrints/Item/DT_Item.DT_Item" (.OutItem (Utilities|Array|Random _outrownames)))
    (:then
      (bind _randomlocation (Class|NavigationSystemV1|GetRandomLocationinNavigableRadius (Transformation|GetActorLocation (Components|GetOwner)) 1e+03 0 0))
      (Game|SpawnActorfromClass (.MemberVar_2 (Utilities|Struct|BreakST_Item _returnvalue)) (Math|Transform|MakeTransform _randomlocation "0, 0, 0" "1.000000,1.000000,1.000000") "Undefined" "MultiplyWithRoot" 0 (Utilities|Struct|MakeST_Item (.MemberVar_0 (Utilities|Struct|BreakST_Item _returnvalue)) (.MemberVar_2 (Utilities|Struct|BreakST_Item _returnvalue))) 0))))