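; Base monster character Blueprint that can deal melee-range damage to the player.
; Capsule overlap with BP_PLayer stores the player and sets IsCanDamage, and end overlap clears both.
; DoDamage applies fixed point-free damage to the stored player without checking the flag, and nothing in this graph calls it.
; An unconnected radial damage node remains as an area-damage alternative.
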(event OnComponentBeginOverlap(CapsuleComponent)
  (params (OverlappedComponent :type Primitive%20Component%20Object%20Reference) (OtherActor :type Actor%20Object%20Reference) (OtherComp :type Primitive%20Component%20Object%20Reference) (OtherBodyIndex :type Integer) (bFromSweep :type Boolean) (SweepResult :type Hit%20Result%20Structure%20%28by%20ref%29))
  (bind _asbp_player (Utilities|Casting|CastToBP_PLayer OtherActor))
  (Variables|Default|SetCharacter _asbp_player)
  (Variables|Default|SetIsCanDamage true))

(event OnComponentEndOverlap(CapsuleComponent)
  (params (OverlappedComponent :type Primitive%20Component%20Object%20Reference) (OtherActor :type Actor%20Object%20Reference) (OtherComp :type Primitive%20Component%20Object%20Reference) (OtherBodyIndex :type Integer))
  (Utilities|Casting|CastToBP_PLayer OtherActor)
  (Variables|Default|SetCharacter 0)
  (Variables|Default|SetIsCanDamage false))

(event EventBeginPlay)

(fn ConstructionScript
  (|CallParentFunction))

(fn DoDamage
  (bind _self self)
  (Game|Damage|ApplyDamage (Variables|Default|GetCharacter) 1e+01 (Pawn|GetController _self) _self))